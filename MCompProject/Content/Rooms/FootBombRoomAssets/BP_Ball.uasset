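; BP_Ball is a timed bomb ball for the FootBomb room that explodes when its fuse runs out.
; The construction script creates a dynamic material, whose Frequency parameter the BallTimer timeline drives from BeginPlay, alongside a separate per-second Time countdown.
; When the timeline finishes, a DoOnce stops physics, spawns BP_BallExplosion and a particle emitter, hides the meshes and destroys the actor after a short delay.
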(event `self.ReceiveBeginPlay`
  ;[1 1 1] Start timer on beginplay
  (`self.ExplosionTimer`)
  (set `self.Time` 9)
  (`KismetSystemLibrary.Delay` 1.0 :!label _label)
  (`/Engine/EditorBlueprintResources/StandardMacros.DecrementInt` (`self.Time`)
    (:`  `
      (goto _label))))

(event `ExplosionTimer`
  ;[1 1 1] Timer for Explosion
  (`MaterialInstanceDynamic.SetScalarParameterValue` (`self.DynamicMaterial`) "Frequency" 0.0)
  (bind (_direction _timer) (`Timeline|BallTimer` :!via `PlayFromStart`)
    (:`Update`
      (`MaterialInstanceDynamic.SetScalarParameterValue` (`self.DynamicMaterial`) "Frequency" _timer))
    (:`Finished`
      (`self.IsBallExploding`))))

(event `IsBallExploding`
  (bind _ball (`self.Ball`))
  (bind _ball_2 (`self.Ball`))
  ;[1 1 1] Spawn Emitter and Particle when timer set Scalar parameter value
  (`/Engine/EditorBlueprintResources/StandardMacros.DoOnce` false
    (:`Completed`
      (`PrimitiveComponent.SetSimulatePhysics` _ball_2 false)
      (`|SpawnActorFromClass` "/Game/Rooms/FootBombRoomAssets/BP_BallExplosion.BP_BallExplosion_C" (`SceneComponent.GetRelativeTransform` _ball_2) "Undefined" "OverrideRootScale" null null)
      (`KismetSystemLibrary.Delay` 0.01)
      (`GameplayStatics.SpawnEmitterAttached` "/Game/Rooms/FootBombRoomAssets/P_BallExplosion.P_BallExplosion" _ball "None" (0.0 0.0 0.0) (struct) (2.0 2.0 2.0) "KeepRelativeOffset" false)
      (`SceneComponent.SetVisibility` _ball false false)
      (`SceneComponent.SetVisibility` (`self.Cylinder`) false false)
      (`SceneComponent.SetVisibility` (`self.Cylinder1`) false false)
      (`KismetSystemLibrary.Delay` 0.5)
      (`self.K2_DestroyActor`))))

(fn `UserConstructionScript`
  (bind _returnvalue (`PrimitiveComponent.CreateDynamicMaterialInstance` (`self.Ball`) 0 "/Game/Rooms/FootBombRoomAssets/Materials/M_Ball.M_Ball"))
  (set `self.DynamicMaterial` _returnvalue))
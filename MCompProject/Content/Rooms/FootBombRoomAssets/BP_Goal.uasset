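; BP_Goal is a goal in the FootbombRoom that scores when a BP_Ball overlaps its collision component.
; A hit destroys the ball and flags the goal as scored, then casts its parent actor to FootbombRoom to decrement the objective count, spawn a new ball and check room completion.
; The goal destroys itself half a second after notifying the room.
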(event `self.Colide.OnComponentBeginOverlap`
  (params (OverlappedComponent :type "PrimitiveComponent Object Reference") (OtherActor :type "Actor Object Reference") (OtherComp :type "PrimitiveComponent Object Reference") (OtherBodyIndex :type Integer) (bFromSweep :type Boolean) (SweepResult :type "HitResult Structure (by ref)"))
  ;[1 1 1] Goal Destroy when scored, minus 1 score and check if room is complete
  (bind _asbp_ball (cast `/Game/Rooms/FootBombRoomAssets/BP_Ball` OtherActor))
  (`self.K2_DestroyActor` _asbp_ball)
  (set `self.HasScored?` true)
  (bind _asfootbomb_room (cast `/Game/Rooms/FootBombRoomAssets/FootbombRoom` (`self.GetParentActor`)))
  (set `/Game/Rooms/FootBombRoomAssets/FootbombRoom.NumberOfObjectives` (- (`/Game/Rooms/FootBombRoomAssets/FootbombRoom.NumberOfObjectives` _asfootbomb_room) 1) _asfootbomb_room)
  (`/Game/Rooms/FootBombRoomAssets/FootbombRoom.SpawnBall` _asfootbomb_room)
  (`/Game/Rooms/FootBombRoomAssets/FootbombRoom.IsRoomComplete` _asfootbomb_room)
  (`KismetSystemLibrary.Delay` 0.5)
  (`self.K2_DestroyActor`))

(fn `UserConstructionScript`)
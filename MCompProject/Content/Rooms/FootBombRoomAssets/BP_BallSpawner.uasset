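; BP_BallSpawner is a spawner for the foot bomb room that keeps producing exploding balls at its own transform.
; BeginPlay spawns the first ball, then loops a roughly five-second Delay into RespawnBall, which calls BallSpawn again.
; Each spawn stores the new BP_Ball and starts its ExplosionTimer.
; DestroySpawnedBall destroys the most recently stored ball but leaves the spawn loop running.
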(event `self.ReceiveBeginPlay`
  ;[1 1 1] BeginPlay event
  (`self.BallSpawn`)
  (`KismetSystemLibrary.Delay` 5.1 :!label _label)
  (`self.RespawnBall`)
  (goto _label))

(event `RespawnBall`
  ;[1 1 1] Respawn Ball CE
  (`self.BallSpawn`))

(event `BallSpawn`
  ;[1 1 1] Spawn Ball CE
  (bind _returnvalue (`|SpawnActorFromClass` "/Game/Rooms/FootBombRoomAssets/BP_Ball.BP_Ball_C" (`self.GetTransform`) "Undefined" "OverrideRootScale" null null))
  (`/Game/Rooms/FootBombRoomAssets/BP_Ball.ExplosionTimer` _returnvalue))

(event `DestroySpawnedBall`
  (`self.K2_DestroyActor` (stale `BallSpawn` _returnvalue)))

(fn `UserConstructionScript`)
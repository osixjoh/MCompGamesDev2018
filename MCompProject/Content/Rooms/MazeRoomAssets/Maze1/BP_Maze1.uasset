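; Maze room Blueprint that spawns two objectives at randomly picked spawn points (possibly the same one) and clears its obstacles once NumberOfObjectives reaches zero.
; MoveWall uses random, non-looping MultiGates to fire timelines that slide four walls along Y, with a WallShift branch for reverse playback.
; Tick polls the count, and completion empties the rotating-wall and button child actors and removes the moving walls' meshes.
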(event `self.ReceiveBeginPlay`
  ;[1 1 1] Begin Play Event
  (`self.SpawnObjective`))

(event `self.ReceiveTick`
  (params (DeltaSeconds :type "Float (single-precision)"))
  ;[1 1 1] Room Complete Check
  (if (<= (`self.Number of Objectives`) 0)
    (`self.RoomIsComplete`)))

(event `RoomIsComplete`
  ;[1 1 1] Destroy Walls and Lever on Room Complete
  (`ChildActorComponent.SetChildActorClass` (`self.RotWall1`) null)
  (`ChildActorComponent.SetChildActorClass` (`self.RotWall2`) null)
  (`ChildActorComponent.SetChildActorClass` (`self.RotWall3`) null)
  (`ChildActorComponent.SetChildActorClass` (`self.RotWall4`) null)
  (`ChildActorComponent.SetChildActorClass` (`self.Button1`) null)
  (`ChildActorComponent.SetChildActorClass` (`self.Button2`) null)
  (`ChildActorComponent.SetChildActorClass` (`self.Button3`) null)
  (`ChildActorComponent.SetChildActorClass` (`self.Button4`) null)
  (`self.DeleteWalls`))

(event `MoveWall`
  (bind _wall1__moveable_ (`self.Wall1 (moveable)`))
  (bind _wall2__moveable_ (`self.Wall2 (moveable)`))
  (bind _wall3__moveable_ (`self.Wall3 (moveable)`))
  (bind _wall4__moveable_ (`self.Wall4 (moveable)`))
  ;[1 1 1] Intitate Movement
  (`|ExecutionSequence`
    (:`then_0`
      (`|MultiGate` true false (`KismetMathLibrary.RandomIntegerInRange` 0 3) :!label _label
        (:`Out 0`
          (bind (_direction _timer_1_float) (`Timeline|Timer 1` :!via `PlayFromStart` :!label _label_2)
            (:`Update`
              (`SceneComponent.K2_SetWorldLocation` _wall1__moveable_ (`KismetMathLibrary.MakeVector` (.x (`SceneComponent.K2_GetComponentLocation` _wall1__moveable_)) (+ (.y (`SceneComponent.K2_GetComponentLocation` _wall1__moveable_)) (`KismetMathLibrary.FClamp` _timer_1_float -6.0 0.0)) (.z (`SceneComponent.K2_GetComponentLocation` _wall1__moveable_))) false false))))
        (:`Out 1`
          (bind (_direction_2 _timer_2_float) (`Timeline|Timer 2` :!via `PlayFromStart` :!label _label_3)
            (:`Update`
              (`SceneComponent.K2_SetWorldLocation` _wall2__moveable_ (`KismetMathLibrary.MakeVector` (.x (`SceneComponent.K2_GetComponentLocation` _wall2__moveable_)) (+ (.y (`SceneComponent.K2_GetComponentLocation` _wall2__moveable_)) (`KismetMathLibrary.FClamp` _timer_2_float -6.0 0.0)) (.z (`SceneComponent.K2_GetComponentLocation` _wall2__moveable_))) false false))))
        (:`Out 2`
          (bind (_direction_3 _timer_3_float) (`Timeline|Timer 3` :!via `PlayFromStart` :!label _label_4)
            (:`Update`
              (`SceneComponent.K2_SetWorldLocation` _wall3__moveable_ (`KismetMathLibrary.MakeVector` (.x (`SceneComponent.K2_GetComponentLocation` _wall3__moveable_)) (+ (.y (`SceneComponent.K2_GetComponentLocation` _wall3__moveable_)) (`KismetMathLibrary.FClamp` _timer_3_float 0.0 6.0)) (.z (`SceneComponent.K2_GetComponentLocation` _wall3__moveable_))) false false))))
        (:`Out 3`
          (bind (_direction_4 _newtrack_3) (`Timeline|Timer 4` :!via `PlayFromStart` :!label _label_5)
            (:`Update`
              (`SceneComponent.K2_SetWorldLocation` _wall4__moveable_ (`KismetMathLibrary.MakeVector` (.x (`SceneComponent.K2_GetComponentLocation` _wall4__moveable_)) (+ (.y (`SceneComponent.K2_GetComponentLocation` _wall4__moveable_)) (`KismetMathLibrary.FClamp` _newtrack_3 0.0 6.0)) (.z (`SceneComponent.K2_GetComponentLocation` _wall4__moveable_))) false false))))))
    (:`then_1`
      (if (`self.WallShift`)
        (`|MultiGate` true false (`KismetMathLibrary.RandomIntegerInRange` 0 3)
          (:`Out 0`
            (goto _label_2 :!via `ReverseFromEnd`))
          (:`Out 1`
            (goto _label_3 :!via `ReverseFromEnd`))
          (:`Out 2`
            (goto _label_4 :!via `ReverseFromEnd`))
          (:`Out 3`
            (goto _label_5 :!via `ReverseFromEnd`)))
        (else
          (goto _label))))))

(fn `DeleteWalls`
  (`StaticMeshComponent.SetStaticMesh` (`self.Wall1 (moveable)`) null)
  (`StaticMeshComponent.SetStaticMesh` (`self.Wall2 (moveable)`) null)
  (`StaticMeshComponent.SetStaticMesh` (`self.Wall3 (moveable)`) null)
  (`StaticMeshComponent.SetStaticMesh` (`self.Wall4 (moveable)`) null))

(fn `SpawnObjective`
  (bind _returnvalue (select `int` (`KismetMathLibrary.RandomIntegerInRange` 0 3) :`0` (`KismetMathLibrary.Conv_VectorToTransform` (`SceneComponent.K2_GetComponentLocation` (`self.ObjectiveSpawn1`))) :`1` (`KismetMathLibrary.Conv_VectorToTransform` (`SceneComponent.K2_GetComponentLocation` (`self.ObjectiveSpawn2`))) :`2` (`KismetMathLibrary.Conv_VectorToTransform` (`SceneComponent.K2_GetComponentLocation` (`self.ObjectiveSpawn3`))) :`3` (`KismetMathLibrary.Conv_VectorToTransform` (`SceneComponent.K2_GetComponentLocation` (`self.ObjectiveSpawn4`)))))
  (`|SpawnActorFromClass` "/Game/Rooms/MazeRoomAssets/Maze1/BP_Maze1Objective.BP_Maze1Objective_C" _returnvalue "Undefined" "OverrideRootScale" null null)
  (`|SpawnActorFromClass` "/Game/Rooms/MazeRoomAssets/Maze1/BP_Maze1Objective.BP_Maze1Objective_C" _returnvalue "Undefined" "OverrideRootScale" null null))

(fn `UserConstructionScript`)
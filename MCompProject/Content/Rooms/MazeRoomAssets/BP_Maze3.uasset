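; BP_Maze3 is a maze room variant that populates itself with walls and objectives on BeginPlay.
; SpawnWalls places a BP_MazeWall at each of eight fixed spawn point locations.
; SpawnObjective acts only when NumberOfObjectives is three, spawning three BP_Objective actors at independently random picks from four spawn points, so positions can repeat.
; The construction script only reassigns PulseRate and NumberOfObjectives to themselves, and PulseRate is otherwise unused here.
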(event `self.ReceiveBeginPlay`
  (`self.SpawnWalls`)
  (`self.SpawnObjective`))

(fn `SpawnObjective`
  (bind _array (`|MakeArray` (`self.ObjectiveSpawn1`) (`self.ObjectiveSpawn2`) (`self.ObjectiveSpawn3`) (`self.ObjectiveSpawn4`)))
  (bind _returnvalue (`SceneComponent.K2_GetComponentToWorld` (`|GetArrayItem` _array (`KismetMathLibrary.RandomIntegerInRange` 0 (- (`KismetArrayLibrary.Array_Length` _array) 1)))))
  (if (== (`self.Number of Objectives`) 3)
    (`|ExecutionSequence`
      (:`then_0`
        (`|SpawnActorFromClass` "/Game/Rooms/MazeRoomAssets/BP_Objective.BP_Objective_C" _returnvalue "Undefined" "OverrideRootScale" null null))
      (:`then_1`
        (`|SpawnActorFromClass` "/Game/Rooms/MazeRoomAssets/BP_Objective.BP_Objective_C" _returnvalue "Undefined" "OverrideRootScale" null null))
      (:`then_2`
        (`|SpawnActorFromClass` "/Game/Rooms/MazeRoomAssets/BP_Objective.BP_Objective_C" _returnvalue "Undefined" "OverrideRootScale" null null)))))

(fn `SpawnWalls`
  (`|ExecutionSequence`
    (:`then_0`
      (`|SpawnActorFromClass` "/Game/Rooms/MazeRoomAssets/BP_MazeWall.BP_MazeWall_C" (`KismetMathLibrary.Conv_VectorToTransform` (`SceneComponent.K2_GetComponentLocation` (`self.SpawnPoint1`))) "Undefined" "OverrideRootScale" null null))
    (:`then_1`
      (`|SpawnActorFromClass` "/Game/Rooms/MazeRoomAssets/BP_MazeWall.BP_MazeWall_C" (`KismetMathLibrary.Conv_VectorToTransform` (`SceneComponent.K2_GetComponentLocation` (`self.SpawnPoint2`))) "Undefined" "OverrideRootScale" null null))
    (:`then_2`
      (`|SpawnActorFromClass` "/Game/Rooms/MazeRoomAssets/BP_MazeWall.BP_MazeWall_C" (`KismetMathLibrary.Conv_VectorToTransform` (`SceneComponent.K2_GetComponentLocation` (`self.SpawnPoint3`))) "Undefined" "OverrideRootScale" null null))
    (:`then_3`
      (`|SpawnActorFromClass` "/Game/Rooms/MazeRoomAssets/BP_MazeWall.BP_MazeWall_C" (`KismetMathLibrary.Conv_VectorToTransform` (`SceneComponent.K2_GetComponentLocation` (`self.SpawnPoint4`))) "Undefined" "OverrideRootScale" null null))
    (:`then_4`
      (`|SpawnActorFromClass` "/Game/Rooms/MazeRoomAssets/BP_MazeWall.BP_MazeWall_C" (`KismetMathLibrary.Conv_VectorToTransform` (`SceneComponent.K2_GetComponentLocation` (`self.SpawnPoint5`))) "Undefined" "OverrideRootScale" null null))
    (:`then_5`
      (`|SpawnActorFromClass` "/Game/Rooms/MazeRoomAssets/BP_MazeWall.BP_MazeWall_C" (`KismetMathLibrary.Conv_VectorToTransform` (`SceneComponent.K2_GetComponentLocation` (`self.SpawnPoint6`))) "Undefined" "OverrideRootScale" null null))
    (:`then_6`
      (`|SpawnActorFromClass` "/Game/Rooms/MazeRoomAssets/BP_MazeWall.BP_MazeWall_C" (`KismetMathLibrary.Conv_VectorToTransform` (`SceneComponent.K2_GetComponentLocation` (`self.SpawnPoint7`))) "Undefined" "OverrideRootScale" null null))
    (:`then_7`
      (`|SpawnActorFromClass` "/Game/Rooms/MazeRoomAssets/BP_MazeWall.BP_MazeWall_C" (`KismetMathLibrary.Conv_VectorToTransform` (`SceneComponent.K2_GetComponentLocation` (`self.SpawnPoint8`))) "Undefined" "OverrideRootScale" null null))))

(fn `UserConstructionScript`
  (set `self.PulseRate` (`self.PulseRate`))
  (set `self.Number of Objectives` (`self.Number of Objectives`)))
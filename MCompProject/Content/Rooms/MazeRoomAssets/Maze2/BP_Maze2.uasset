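; Maze room Blueprint with shifting walls that spawns two objectives at random picks from five points on BeginPlay.
; WallMove uses a random non-looping MultiGate to play one of eight timelines, each adding offsets to a wall's world X or Y.
; ResetWalls reverses timelines through its own random gate, so picks are independent.
; Tick polls NumberOfObjectives and, at zero, clears rotating-wall and button child actors plus moving-wall meshes.
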(event `self.ReceiveBeginPlay`
  ;[1 1 1] Begin Play Event
  (`self.SpawnObjective`))

(event `self.ReceiveTick`
  (params (DeltaSeconds :type "Float (single-precision)"))
  ;[1 1 1] Room Complete Check
  (if (<= (`self.Number of Objectives`) 0)
    (`self.RoomIsComplete`)))

(event `RoomIsComplete`
  ;[1 1 1] Destroy Walls and Lever on Room Complete
  (`ChildActorComponent.SetChildActorClass` (`self.RotWall1`) null)
  (`ChildActorComponent.SetChildActorClass` (`self.RotWall2`) null)
  (`ChildActorComponent.SetChildActorClass` (`self.RotWall3`) null)
  (`ChildActorComponent.SetChildActorClass` (`self.RotWall4`) null)
  (`ChildActorComponent.SetChildActorClass` (`self.RotWall5`) null)
  (`ChildActorComponent.SetChildActorClass` (`self.RotWall6`) null)
  (`ChildActorComponent.SetChildActorClass` (`self.Button1`) null)
  (`ChildActorComponent.SetChildActorClass` (`self.Button2`) null)
  (`ChildActorComponent.SetChildActorClass` (`self.Button3`) null)
  (`ChildActorComponent.SetChildActorClass` (`self.Button4`) null)
  (`self.DeleteWalls`))

(event `WallMove`
  (bind _wally3__moveable_ (`self.WallY3 (moveable)`))
  (bind _wally4__moveable_ (`self.WallY4 (moveable)`))
  (bind _wally1__moveable_ (`self.WallY1 (moveable)`))
  (bind _wally2__moveable_ (`self.WallY2 (moveable)`))
  (bind _wallx1__moveable_ (`self.WallX1 (moveable)`))
  (bind _wallx2__moveable_ (`self.WallX2 (moveable)`))
  (bind _wallx3__moveable_ (`self.WallX3 (moveable)`))
  (bind _wallx4__moveable_ (`self.WallX4 (moveable)`))
  ;[1 1 1] Intitate Movement
  (`|MultiGate` true false (`KismetMathLibrary.RandomIntegerInRange` 0 7)
    (:`Out 0`
      (bind (_direction _timer_1) (`Timeline|Timer 1` :!via `PlayFromStart` :!label _label)
        (:`Update`
          (`SceneComponent.K2_SetWorldLocation` _wally1__moveable_ (`KismetMathLibrary.MakeVector` (.x (`SceneComponent.K2_GetComponentLocation` _wally1__moveable_)) (+ (.y (`SceneComponent.K2_GetComponentLocation` _wally1__moveable_)) _timer_1) (.z (`SceneComponent.K2_GetComponentLocation` _wally1__moveable_))) false false))))
    (:`Out 1`
      (bind (_direction_2 _timer_2) (`Timeline|Timer 2` :!via `PlayFromStart` :!label _label_2)
        (:`Update`
          (`SceneComponent.K2_SetWorldLocation` _wally2__moveable_ (`KismetMathLibrary.MakeVector` (.x (`SceneComponent.K2_GetComponentLocation` _wally2__moveable_)) (+ (.y (`SceneComponent.K2_GetComponentLocation` _wally2__moveable_)) _timer_2) (.z (`SceneComponent.K2_GetComponentLocation` _wally2__moveable_))) false false))))
    (:`Out 2`
      (bind (_direction_3 _timer_3) (`Timeline|Timer 3` :!via `PlayFromStart` :!label _label_3)
        (:`Update`
          (`SceneComponent.K2_SetWorldLocation` _wally3__moveable_ (`KismetMathLibrary.MakeVector` (.x (`SceneComponent.K2_GetComponentLocation` _wally3__moveable_)) (+ (.y (`SceneComponent.K2_GetComponentLocation` _wally3__moveable_)) _timer_3) (.z (`SceneComponent.K2_GetComponentLocation` _wally3__moveable_))) false false))))
    (:`Out 3`
      (bind (_direction_4 _timer_4) (`Timeline|Timer 4` :!via `PlayFromStart` :!label _label_4)
        (:`Update`
          (`SceneComponent.K2_SetWorldLocation` _wally4__moveable_ (`KismetMathLibrary.MakeVector` (.x (`SceneComponent.K2_GetComponentLocation` _wally4__moveable_)) (+ (.y (`SceneComponent.K2_GetComponentLocation` _wally4__moveable_)) _timer_4) (.z (`SceneComponent.K2_GetComponentLocation` _wally4__moveable_))) false false))))
    (:`Out 4`
      (bind (_direction_5 _timer_5) (`Timeline|Timer 5` :!via `PlayFromStart` :!label _label_5)
        (:`Update`
          (`SceneComponent.K2_SetWorldLocation` _wallx1__moveable_ (`KismetMathLibrary.MakeVector` (+ (.x (`SceneComponent.K2_GetComponentLocation` _wallx1__moveable_)) _timer_5) (.y (`SceneComponent.K2_GetComponentLocation` _wallx1__moveable_)) (.z (`SceneComponent.K2_GetComponentLocation` _wallx1__moveable_))) false false))))
    (:`Out 5`
      (bind (_direction_6 _timer_6) (`Timeline|Timer 6` :!via `PlayFromStart` :!label _label_6)
        (:`Update`
          (`SceneComponent.K2_SetWorldLocation` _wallx2__moveable_ (`KismetMathLibrary.MakeVector` (+ (.x (`SceneComponent.K2_GetComponentLocation` _wallx2__moveable_)) _timer_6) (.y (`SceneComponent.K2_GetComponentLocation` _wallx2__moveable_)) (.z (`SceneComponent.K2_GetComponentLocation` _wallx2__moveable_))) false false))))
    (:`Out 6`
      (bind (_direction_7 _timer) (`Timeline|Timer 7` :!via `PlayFromStart` :!label _label_7)
        (:`Update`
          (`SceneComponent.K2_SetWorldLocation` _wallx3__moveable_ (`KismetMathLibrary.MakeVector` (+ (.x (`SceneComponent.K2_GetComponentLocation` _wallx3__moveable_)) _timer) (.y (`SceneComponent.K2_GetComponentLocation` _wallx3__moveable_)) (.z (`SceneComponent.K2_GetComponentLocation` _wallx3__moveable_))) false false))))
    (:`Out 7`
      (bind (_direction_8 _timer_8) (`Timeline|Timer 8` :!via `PlayFromStart` :!label _label_8)
        (:`Update`
          (`SceneComponent.K2_SetWorldLocation` _wallx4__moveable_ (`KismetMathLibrary.MakeVector` (+ (.x (`SceneComponent.K2_GetComponentLocation` _wallx4__moveable_)) _timer_8) (.y (`SceneComponent.K2_GetComponentLocation` _wallx4__moveable_)) (.z (`SceneComponent.K2_GetComponentLocation` _wallx4__moveable_))) false false))))))

(event `ResetWalls`
  ;[1 1 1] Intitate Movement
  (`|MultiGate` true false (`KismetMathLibrary.RandomIntegerInRange` 0 7)
    (:`Out 0`
      (goto _label :!via `ReverseFromEnd`))
    (:`Out 1`
      (goto _label_2 :!via `ReverseFromEnd`))
    (:`Out 2`
      (goto _label_3 :!via `ReverseFromEnd`))
    (:`Out 3`
      (goto _label_4 :!via `ReverseFromEnd`))
    (:`Out 4`
      (goto _label_5 :!via `ReverseFromEnd`))
    (:`Out 5`
      (goto _label_6 :!via `ReverseFromEnd`))
    (:`Out 6`
      (goto _label_7 :!via `ReverseFromEnd`))
    (:`Out 7`
      (goto _label_8 :!via `ReverseFromEnd`))))

(fn `DeleteWalls`
  (`StaticMeshComponent.SetStaticMesh` (`self.WallX1 (moveable)`) null)
  (`StaticMeshComponent.SetStaticMesh` (`self.WallX2 (moveable)`) null)
  (`StaticMeshComponent.SetStaticMesh` (`self.WallX3 (moveable)`) null)
  (`StaticMeshComponent.SetStaticMesh` (`self.WallX4 (moveable)`) null)
  (`StaticMeshComponent.SetStaticMesh` (`self.WallY1 (moveable)`) null)
  (`StaticMeshComponent.SetStaticMesh` (`self.WallY2 (moveable)`) null)
  (`StaticMeshComponent.SetStaticMesh` (`self.WallY3 (moveable)`) null)
  (`StaticMeshComponent.SetStaticMesh` (`self.WallY4 (moveable)`) null))

(fn `SpawnObjective`
  (bind _returnvalue (select `int` (`KismetMathLibrary.RandomIntegerInRange` 0 4) :`0` (`KismetMathLibrary.Conv_VectorToTransform` (`SceneComponent.K2_GetComponentLocation` (`self.ObjectiveSpawn1`))) :`1` (`KismetMathLibrary.Conv_VectorToTransform` (`SceneComponent.K2_GetComponentLocation` (`self.ObjectiveSpawn2`))) :`2` (`KismetMathLibrary.Conv_VectorToTransform` (`SceneComponent.K2_GetComponentLocation` (`self.ObjectiveSpawn3`))) :`3` (`KismetMathLibrary.Conv_VectorToTransform` (`SceneComponent.K2_GetComponentLocation` (`self.ObjectiveSpawn4`))) :`4` (`KismetMathLibrary.Conv_VectorToTransform` (`SceneComponent.K2_GetComponentLocation` (`self.ObjectiveSpawn5`)))))
  (`|SpawnActorFromClass` "/Game/Rooms/MazeRoomAssets/Maze2/BP_Maze2Objective.BP_Maze2Objective_C" _returnvalue "Undefined" "OverrideRootScale" null null)
  (`|SpawnActorFromClass` "/Game/Rooms/MazeRoomAssets/Maze2/BP_Maze2Objective.BP_Maze2Objective_C" _returnvalue "Undefined" "OverrideRootScale" null null))

(fn `UserConstructionScript`)
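; BP_MazeLever2 is the second lever in the maze room, activating walls when the top-down character overlaps its trigger.
; It calls Lever2 on its parent MazeRoom actor, then reverses levers 1, 3 and 4 if the room flags them as pressed.
; When the character leaves, the trigger stops generating overlap events for a short delay before re-arming.
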(event `self.Trigger.OnComponentBeginOverlap`
  (params (OverlappedComponent :type "PrimitiveComponent Object Reference") (OtherActor :type "Actor Object Reference") (OtherComp :type "PrimitiveComponent Object Reference") (OtherBodyIndex :type Integer) (bFromSweep :type Boolean) (SweepResult :type "HitResult Structure (by ref)"))
  ;[1 1 1] Activate Walls
  (cast `/Game/TopDownCharacter` OtherActor)
  (bind _asmaze_room (cast `/Game/Rooms/MazeRoomAssets/MazeRoom` (`self.GetParentActor`)))
  (`/Game/Rooms/MazeRoomAssets/MazeRoom.Lever 2` _asmaze_room)
  (`|ExecutionSequence`
    (:`then_0`
      (if (`/Game/Rooms/MazeRoomAssets/MazeRoom.Lever1Pressed?` _asmaze_room)
        (`/Game/Rooms/MazeRoomAssets/MazeRoom.Lever 1 Reverse` _asmaze_room)))
    (:`then_1`
      (if (`/Game/Rooms/MazeRoomAssets/MazeRoom.Lever3Pressed?` _asmaze_room)
        (`/Game/Rooms/MazeRoomAssets/MazeRoom.Lever 3 Reverse` _asmaze_room)))
    (:`then_2`
      (if (`/Game/Rooms/MazeRoomAssets/MazeRoom.Lever4Pressed?` _asmaze_room)
        (`/Game/Rooms/MazeRoomAssets/MazeRoom.Lever 4 Reverse` _asmaze_room)))))

(event `self.Trigger.OnComponentEndOverlap`
  (params (OverlappedComponent :type "PrimitiveComponent Object Reference") (OtherActor :type "Actor Object Reference") (OtherComp :type "PrimitiveComponent Object Reference") (OtherBodyIndex :type Integer))
  ;[1 1 1] Reset Lever
  (cast `/Game/TopDownCharacter` OtherActor)
  (`self.TriggerDeactiveDelayed`))

(event `TriggerDeactiveDelayed`
  (bind _trigger (`self.Trigger`))
  ;[1 1 1] Reset Lever
  (set `PrimitiveComponent.bGenerateOverlapEvents` false _trigger)
  (`KismetSystemLibrary.Delay` 1.0)
  (set `PrimitiveComponent.bGenerateOverlapEvents` true _trigger))

(fn `UserConstructionScript`)
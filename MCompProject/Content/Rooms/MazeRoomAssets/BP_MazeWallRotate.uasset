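; BP_MazeWallRotate is a maze room wall that turns in timed steps through RotatePlus and RotateMinus events.
; Each trigger activates a RotatingMovement component, waits one second on a Delay, then deactivates it.
; Helper events set a positive or negative 90 degree-per-second rate on one axis, so a step is roughly a quarter turn.
; The turn relies on timing, with no snap to a target angle.
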(event `RotatePlus`
  ;[1 1 1] Rotation Triggers
  (`self.RotMove+`)
  (`self.RotMove1`)
  (`KismetSystemLibrary.Delay` 1.0)
  (`self.RotMove0`))

(event `RotateMinus`
  ;[1 1 1] Rotation Triggers
  (`self.RotMove-`)
  (`self.RotMove1`)
  (`KismetSystemLibrary.Delay` 1.0)
  (`self.RotMove0`))

(event `RotMove1`
  ;[1 1 1] Rotation Triggers
  (`ActorComponent.SetActive` (`self.RotatingMovement`) true false))

(event `RotMove+`
  ;[1 1 1] Rotation Triggers
  (set `RotatingMovementComponent.RotationRate` (`KismetMathLibrary.MakeRotator` 0.0 0.0 (`KismetMathLibrary.FClamp` 90.0 0.0 90.0)) (`self.RotatingMovement`)))

(event `RotMove0`
  ;[1 1 1] Rotation Triggers
  (`ActorComponent.SetActive` (`self.RotatingMovement`) false false))

(event `RotMove-`
  ;[1 1 1] Rotation Triggers
  (set `RotatingMovementComponent.RotationRate` (`KismetMathLibrary.MakeRotator` 0.0 0.0 (`KismetMathLibrary.FClamp` -90.0 -90.0 0.0)) (`self.RotatingMovement`)))

(fn `UserConstructionScript`)
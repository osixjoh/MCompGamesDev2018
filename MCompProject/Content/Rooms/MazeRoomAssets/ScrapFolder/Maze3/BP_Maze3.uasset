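; Scrapped-looking maze room with movable walls and objectives, currently inert because every event is empty and its logic is disconnected.
; The unwired graph spawns two objectives at random points and uses random MultiGates to play or reverse timelines that slide eight walls along X or Y.
; An unwired completion check on the objective count leads to helpers that clear wall meshes and child-actor rotating walls and buttons.
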(event `self.ReceiveBeginPlay`
  ;[1 1 1] Begin Play Event
)

(event `self.ReceiveTick`
  (params (DeltaSeconds :type "Float (single-precision)"))
  ;[1 1 1] Room Complete Check
)

(event `RoomIsComplete`
  ;[1 1 1] Destroy Walls and Lever on Room Complete
)

(event `WallMove`
  ;[1 1 1] Intitate Movement
)

(event `ResetWalls`
  ;[1 1 1] Intitate Movement
)

(fn `DeleteWalls`
  (`StaticMeshComponent.SetStaticMesh` (`self.WallX1 (moveable)`) null)
  (`StaticMeshComponent.SetStaticMesh` (`self.WallX2 (moveable)`) null)
  (`StaticMeshComponent.SetStaticMesh` (`self.WallX3 (moveable)`) null)
  (`StaticMeshComponent.SetStaticMesh` (`self.WallX4 (moveable)`) null)
  (`StaticMeshComponent.SetStaticMesh` (`self.WallY1 (moveable)`) null)
  (`StaticMeshComponent.SetStaticMesh` (`self.WallY2 (moveable)`) null)
  (`StaticMeshComponent.SetStaticMesh` (`self.WallY3 (moveable)`) null)
  (`StaticMeshComponent.SetStaticMesh` (`self.WallY4 (moveable)`) null))

(fn `DestroyActors`
  (`ChildActorComponent.SetChildActorClass` (`self.RotWall1`) null)
  (`ChildActorComponent.SetChildActorClass` (`self.RotWall2`) null)
  (`ChildActorComponent.SetChildActorClass` (`self.RotWall3`) null)
  (`ChildActorComponent.SetChildActorClass` (`self.RotWall4`) null)
  (`ChildActorComponent.SetChildActorClass` (`self.Button1`) null)
  (`ChildActorComponent.SetChildActorClass` (`self.Button2`) null)
  (`ChildActorComponent.SetChildActorClass` (`self.Button3`) null)
  (`ChildActorComponent.SetChildActorClass` (`self.Button4`) null)
  (`ChildActorComponent.SetChildActorClass` (`self.RotWall5`) null)
  (`ChildActorComponent.SetChildActorClass` (`self.RotWall6`) null))

(fn `SpawnObjective`
  (bind _returnvalue (select `int` (`KismetMathLibrary.RandomIntegerInRange` 0 4) :`0` (`KismetMathLibrary.Conv_VectorToTransform` (`SceneComponent.K2_GetComponentLocation` (`self.ObjectiveSpawn1`))) :`1` (`KismetMathLibrary.Conv_VectorToTransform` (`SceneComponent.K2_GetComponentLocation` (`self.ObjectiveSpawn2`))) :`2` (`KismetMathLibrary.Conv_VectorToTransform` (`SceneComponent.K2_GetComponentLocation` (`self.ObjectiveSpawn3`))) :`3` (`KismetMathLibrary.Conv_VectorToTransform` (`SceneComponent.K2_GetComponentLocation` (`self.ObjectiveSpawn4`))) :`4` (`KismetMathLibrary.Conv_VectorToTransform` (`SceneComponent.K2_GetComponentLocation` (`self.ObjectiveSpawn5`)))))
  (`|SpawnActorFromClass` "/Game/Rooms/MazeRoomAssets/ScrapFolder/Maze3/BP_Maze3Objective.BP_Maze3Objective_C" _returnvalue "Undefined" "OverrideRootScale" null null)
  (`|SpawnActorFromClass` "/Game/Rooms/MazeRoomAssets/ScrapFolder/Maze3/BP_Maze3Objective.BP_Maze3Objective_C" _returnvalue "Undefined" "OverrideRootScale" null null))

(fn `UserConstructionScript`)
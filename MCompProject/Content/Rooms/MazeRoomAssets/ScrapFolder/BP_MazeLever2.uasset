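; Maze lever, placed as a child actor of MazeRoom2, that the TopDownCharacter triggers by overlap to alter the room.
; Overlap plays a timeline pitching the lever, then a looping random MultiGate calls the room's rotate, move or scale master trigger.
; Ending overlap reverses the lever and disables trigger overlaps for one second.
; The timeline update sets pitch to base plus, then base minus, its value, so only the latter sticks.
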(event `self.Trigger.OnComponentBeginOverlap`
  (params (OverlappedComponent :type "PrimitiveComponent Object Reference") (OtherActor :type "Actor Object Reference") (OtherComp :type "PrimitiveComponent Object Reference") (OtherBodyIndex :type Integer) (bFromSweep :type Boolean) (SweepResult :type "HitResult Structure (by ref)"))
  ;[1 1 1] Activate Walls
  (cast `/Game/TopDownCharacter` OtherActor)
  (`self.DoLeverAnim`)
  (bind _asmaze_room_2 (cast `/Game/Rooms/MazeRoomAssets/ScrapFolder/MazeRoom2` (`self.GetParentActor`)))
  (`|MultiGate` true true (`KismetMathLibrary.RandomIntegerInRange` 0 2)
    (:`Out 0`
      (`/Game/Rooms/MazeRoomAssets/ScrapFolder/MazeRoom2.Rotate Master Trigger` _asmaze_room_2))
    (:`Out 1`
      (`/Game/Rooms/MazeRoomAssets/ScrapFolder/MazeRoom2.Move Master Trigger` _asmaze_room_2))
    (:`Out 2`
      (`/Game/Rooms/MazeRoomAssets/ScrapFolder/MazeRoom2.Scale Master Trigger` _asmaze_room_2))))

(event `DoLeverAnim`
  (bind _lever (`self.Lever`))
  (bind (_baseleverrotator_roll _baseleverrotator_pitch) (`KismetMathLibrary.BreakRotator` (`self.BaseLeverRotator`)))
  ;[1 1 1] Lever Animation Set
  (bind (_direction _timer) (`Timeline|Lever Rotation Timer` :!via `PlayFromStart` :!label _label)
    (:`Update`
      (`|ExecutionSequence`
        (:`then_0`
          (`SceneComponent.K2_SetRelativeRotation` _lever (`KismetMathLibrary.MakeRotator` 0.0 (+ _baseleverrotator_pitch _timer)) false false))
        (:`then_1`
          (`SceneComponent.K2_SetRelativeRotation` _lever (`KismetMathLibrary.MakeRotator` 0.0 (- _baseleverrotator_pitch _timer)) false false))))))

(event `ResetLever`
  ;[1 1 1] Lever Animation Set
  (goto _label :!via `ReverseFromEnd`))

(event `self.Trigger.OnComponentEndOverlap`
  (params (OverlappedComponent :type "PrimitiveComponent Object Reference") (OtherActor :type "Actor Object Reference") (OtherComp :type "PrimitiveComponent Object Reference") (OtherBodyIndex :type Integer))
  ;[1 1 1] Reset Lever
  (cast `/Game/TopDownCharacter` OtherActor)
  (`self.TriggerDeactiveDelayed`)
  (`self.ResetLever`)
  (`KismetSystemLibrary.Delay` 1.0))

(event `TriggerDeactiveDelayed`
  (bind _trigger (`self.Trigger`))
  ;[1 1 1] Reset Lever
  (set `PrimitiveComponent.bGenerateOverlapEvents` false _trigger)
  (`KismetSystemLibrary.Delay` 1.0)
  (set `PrimitiveComponent.bGenerateOverlapEvents` true _trigger))

(fn `UserConstructionScript`)
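; Lever for the Maze2 room that shuffles the maze when a TopDownCharacter enters its trigger.
; Overlap plays a timeline that pitches the lever, then loops over all BP_Maze2 and, nested inside, all BP_MazeWallRotate actors.
; Random looping MultiGates choose WallMove or ResetWalls, and RotatePlus or RotateMinus, on each inner iteration.
; Leaving the trigger reverses the lever after a delay and briefly disables overlap events as a cooldown.
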(event `self.Trigger.OnComponentBeginOverlap`
  (params (OverlappedComponent :type "PrimitiveComponent Object Reference") (OtherActor :type "Actor Object Reference") (OtherComp :type "PrimitiveComponent Object Reference") (OtherBodyIndex :type Integer) (bFromSweep :type Boolean) (SweepResult :type "HitResult Structure (by ref)"))
  ;[1 1 1] Activate Walls
  (cast `/Game/TopDownCharacter` OtherActor)
  (`self.DoLeverAnim`)
  (bind _outactors (`GameplayStatics.GetAllActorsOfClass` "/Game/Rooms/MazeRoomAssets/ScrapFolder/Maze2/BP_Maze2.BP_Maze2_C"))
  (for _array_element _outactors
    (bind _outactors_2 (`GameplayStatics.GetAllActorsOfClass` "/Game/Rooms/MazeRoomAssets/BP_MazeWallRotate.BP_MazeWallRotate_C"))
    (for _array_element_2 _outactors_2
      (`|ExecutionSequence`
        (:`then_0`
          (`|MultiGate` true true (`KismetMathLibrary.RandomIntegerInRange` 0 1)
            (:`Out 0`
              (`/Game/Rooms/MazeRoomAssets/ScrapFolder/Maze2/BP_Maze2.WallMove` _array_element))
            (:`Out 1`
              (`/Game/Rooms/MazeRoomAssets/ScrapFolder/Maze2/BP_Maze2.ResetWalls` _array_element))))
        (:`then_1`
          (`|MultiGate` true true (`KismetMathLibrary.RandomIntegerInRange` 0 1)
            (:`Out 0`
              (`/Game/Rooms/MazeRoomAssets/BP_MazeWallRotate.RotatePlus` _array_element_2))
            (:`Out 1`
              (`/Game/Rooms/MazeRoomAssets/BP_MazeWallRotate.RotateMinus` _array_element_2))))))))

(event `DoLeverAnim`
  (bind _lever (`self.Lever`))
  (bind (_baseleverrotator_roll _baseleverrotator_pitch) (`KismetMathLibrary.BreakRotator` (`self.BaseLeverRotator`)))
  ;[1 1 1] Lever Animation Set
  (bind (_direction _rotator) (`Timeline|TimerLeverSet` :!label _label)
    (:`Update`
      (`|ExecutionSequence`
        (:`then_0`
          (`SceneComponent.K2_SetRelativeRotation` _lever (`KismetMathLibrary.MakeRotator` 0.0 (+ _baseleverrotator_pitch _rotator)) false false))
        (:`then_1`
          (`SceneComponent.K2_SetRelativeRotation` _lever (`KismetMathLibrary.MakeRotator` 0.0 (- 120.0 _rotator)) false false)
          (`SceneComponent.K2_SetRelativeRotation` (`self.Lever`) (`KismetMathLibrary.MakeRotator` 0.0 (- 120.0 _rotator)) false false))))))

(event `self.Trigger.OnComponentEndOverlap`
  (params (OverlappedComponent :type "PrimitiveComponent Object Reference") (OtherActor :type "Actor Object Reference") (OtherComp :type "PrimitiveComponent Object Reference") (OtherBodyIndex :type Integer))
  ;[1 1 1] Reset Lever
  (cast `/Game/TopDownCharacter` OtherActor)
  (`KismetSystemLibrary.Delay` 1.0)
  (`self.TriggerDeactiveDelayed`)
  (`self.ResetLever`))

(event `ResetLever`
  ;[1 1 1] Lever Animation Set
  (goto _label :!via `Reverse`))

(event `TriggerDeactiveDelayed`
  (bind _trigger (`self.Trigger`))
  ;[1 1 1] Reset Lever
  (set `PrimitiveComponent.bGenerateOverlapEvents` false _trigger)
  (`KismetSystemLibrary.Delay` 1.0)
  (set `PrimitiveComponent.bGenerateOverlapEvents` true _trigger))

(fn `UserConstructionScript`)
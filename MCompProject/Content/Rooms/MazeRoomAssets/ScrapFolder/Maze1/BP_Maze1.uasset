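; Maze room that spawns two objectives at random picks from four spawn points and manages four sliding walls.
; MoveWall and ResetWall use separate random, non-looping MultiGates to play or reverse one wall's timeline, offsetting it along Y.
; Tick watches NumberOfObjectives; at zero it clears wall meshes and rotating-wall and button child actors, then calls RoomComplete on a MazeMasterRef entry indexed by array length.
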(event `WhenRoomIsComplete`
  ;[1 1 1] Destroy Walls and Lever on Room Complete
  (`self.DestroyActors`)
  (`self.DeleteWalls`))

(event `self.ReceiveBeginPlay`
  (`self.SpawnObjective`))

(event `self.ReceiveTick`
  (params (DeltaSeconds :type "Float (single-precision)"))
  (bind _mazemasterref (`self.MazeMasterRef`))
  (if (== (`self.Number of Objectives`) 0)
    (`self.WhenRoomIsComplete`)
    (`/Game/Rooms/MasterRoom/MasterRoom.Room Complete` (`|GetArrayItem` _mazemasterref (`KismetArrayLibrary.Array_Length` _mazemasterref)))))

(event `MoveWall`
  (bind _wall1__moveable_ (`self.Wall1 (moveable)`))
  (bind _wall2__moveable_ (`self.Wall2 (moveable)`))
  (bind _wall3__moveable_ (`self.Wall3 (moveable)`))
  (bind _wall4__moveable_ (`self.Wall4 (moveable)`))
  ;[1 1 1] Intitate Movement
  (`|MultiGate` true false (`KismetMathLibrary.RandomIntegerInRange` 0 3)
    (:`Out 0`
      (bind (_direction _timer_1_float) (`Timeline|Timer 1` :!via `PlayFromStart` :!label _label)
        (:`Update`
          (`SceneComponent.K2_SetWorldLocation` _wall1__moveable_ (`KismetMathLibrary.MakeVector` (.x (`SceneComponent.K2_GetComponentLocation` _wall1__moveable_)) (+ (.y (`SceneComponent.K2_GetComponentLocation` _wall1__moveable_)) _timer_1_float) (.z (`SceneComponent.K2_GetComponentLocation` _wall1__moveable_))) false false))))
    (:`Out 1`
      (bind (_direction_2 _timer_2_float) (`Timeline|Timer 2` :!via `PlayFromStart` :!label _label_2)
        (:`Update`
          (`SceneComponent.K2_SetWorldLocation` _wall2__moveable_ (`KismetMathLibrary.MakeVector` (.x (`SceneComponent.K2_GetComponentLocation` _wall2__moveable_)) (+ (.y (`SceneComponent.K2_GetComponentLocation` _wall2__moveable_)) _timer_2_float) (.z (`SceneComponent.K2_GetComponentLocation` _wall2__moveable_))) false false))))
    (:`Out 2`
      (bind (_direction_3 _timer_3_float) (`Timeline|Timer 3` :!via `PlayFromStart` :!label _label_3)
        (:`Update`
          (`SceneComponent.K2_SetWorldLocation` _wall3__moveable_ (`KismetMathLibrary.MakeVector` (.x (`SceneComponent.K2_GetComponentLocation` _wall3__moveable_)) (+ (.y (`SceneComponent.K2_GetComponentLocation` _wall3__moveable_)) _timer_3_float) (.z (`SceneComponent.K2_GetComponentLocation` _wall3__moveable_))) false false))))
    (:`Out 3`
      (bind (_direction_4 _newtrack_3) (`Timeline|Timer 4` :!via `PlayFromStart` :!label _label_4)
        (:`Update`
          (`SceneComponent.K2_SetWorldLocation` _wall4__moveable_ (`KismetMathLibrary.MakeVector` (.x (`SceneComponent.K2_GetComponentLocation` _wall4__moveable_)) (+ (.y (`SceneComponent.K2_GetComponentLocation` _wall4__moveable_)) _newtrack_3) (.z (`SceneComponent.K2_GetComponentLocation` _wall4__moveable_))) false false))))))

(event `ResetWall`
  ;[1 1 1] Intitate Movement
  (`|MultiGate` true false (`KismetMathLibrary.RandomIntegerInRange` 0 3)
    (:`Out 0`
      (goto _label :!via `ReverseFromEnd`))
    (:`Out 1`
      (goto _label_2 :!via `ReverseFromEnd`))
    (:`Out 2`
      (goto _label_3 :!via `ReverseFromEnd`))
    (:`Out 3`
      (goto _label_4 :!via `ReverseFromEnd`))))

(fn `DeleteWalls`
  (`StaticMeshComponent.SetStaticMesh` (`self.Wall1 (moveable)`) null)
  (`StaticMeshComponent.SetStaticMesh` (`self.Wall2 (moveable)`) null)
  (`StaticMeshComponent.SetStaticMesh` (`self.Wall3 (moveable)`) null)
  (`StaticMeshComponent.SetStaticMesh` (`self.Wall4 (moveable)`) null))

(fn `DestroyActors`
  (`ChildActorComponent.SetChildActorClass` (`self.RotWall1`) null)
  (`ChildActorComponent.SetChildActorClass` (`self.RotWall2`) null)
  (`ChildActorComponent.SetChildActorClass` (`self.RotWall3`) null)
  (`ChildActorComponent.SetChildActorClass` (`self.RotWall4`) null)
  (`ChildActorComponent.SetChildActorClass` (`self.Button1`) null)
  (`ChildActorComponent.SetChildActorClass` (`self.Button2`) null)
  (`ChildActorComponent.SetChildActorClass` (`self.Button3`) null)
  (`ChildActorComponent.SetChildActorClass` (`self.Button4`) null))

(fn `SpawnObjective`
  (bind _returnvalue (select `int` (`KismetMathLibrary.RandomIntegerInRange` 0 3) :`0` (`KismetMathLibrary.Conv_VectorToTransform` (`SceneComponent.K2_GetComponentLocation` (`self.ObjectiveSpawn1`))) :`1` (`KismetMathLibrary.Conv_VectorToTransform` (`SceneComponent.K2_GetComponentLocation` (`self.ObjectiveSpawn2`))) :`2` (`KismetMathLibrary.Conv_VectorToTransform` (`SceneComponent.K2_GetComponentLocation` (`self.ObjectiveSpawn3`))) :`3` (`KismetMathLibrary.Conv_VectorToTransform` (`SceneComponent.K2_GetComponentLocation` (`self.ObjectiveSpawn4`)))))
  (`|SpawnActorFromClass` "/Game/Rooms/MazeRoomAssets/BP_MazeObjective.BP_MazeObjective_C" _returnvalue "Undefined" "OverrideRootScale" null null)
  (`|SpawnActorFromClass` "/Game/Rooms/MazeRoomAssets/BP_MazeObjective.BP_MazeObjective_C" _returnvalue "Undefined" "OverrideRootScale" null null)
  (set `self.Number of Objectives` 2))

(fn `UserConstructionScript`)